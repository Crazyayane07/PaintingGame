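; BP_Mosaic is a player's paintable mosaic board in the painting game, labeled with that player's nickname.
; A server event spawns and attaches a square grid of BP_MosaicTile actors sized by BP_GameManager, multicasting the label's text and height.
; It scores tile colors against the manager's reversed target mosaic and fires OnFinPainting when all match.
; A server clear event multicasts a reset to every tile.
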(event `self.ReceiveBeginPlay`
  (`self.Server_SetUp`))

(event `Server_SetUp`
  (`self.GenerateTiles`)
  (bind _asbp_player (cast `/Game/PaintingGame/Blueprints/Player/BP_Player` (`PlayerState.GetPawn` (`self.PlayerStateRef`))))
  (`self.Multicast_SetText` (`/Game/PaintingGame/Blueprints/Player/BP_Player.GetNickname` _asbp_player)))

(event `Multicast_SetText`
  (params (Nickname :type String))
  (`TextRenderComponent.K2_SetText` (`self.TextRender`) (`KismetTextLibrary.Conv_StringToText` Nickname)))

(event `Multicast_SetTextLocation`
  (params (Row :type Integer))
  (`SceneComponent.K2_SetRelativeLocation` (`self.TextRender`) (`KismetMathLibrary.MakeVector` 0.0 0.0 (`KismetMathLibrary.Conv_IntToDouble` (* Row (`self.TilesOffset`)))) false false))

(event `Server_Clear`
  (for _array_element (`self.Tiles`)
    (`/Game/PaintingGame/Blueprints/Objects/Mosaic/BP_MosaicTile.Multicast_Clear` _array_element)))

(fn `CalculatePoints`
  (returns (Points :type Integer))
  (locals (TilePoints :type Integer :default 0) (TargetMosaic :type "Array of Integer"))
  (set `local.TilePoints` 0)
  (bind _returnvalue (`GameplayStatics.GetActorOfClass` "/Game/PaintingGame/Blueprints/Game/BP_GameManager.BP_GameManager_C"))
  (bind _output_get (set `local.TargetMosaic` (`PGGameManager.GetMosaic` _returnvalue)))
  (`KismetArrayLibrary.Array_Reverse` _output_get)
  (for (_array_element _array_index) (`self.Tiles`)
    (if (== (`|GetArrayItem` (`local.TargetMosaic`) _array_index) (`/Game/PaintingGame/Blueprints/Objects/BP_ColorableObject.ColorId` _array_element))
      (`/Engine/EditorBlueprintResources/StandardMacros.IncrementInt` (`local.TilePoints`))))
  (return (`local.TilePoints`)))

(fn `CheckIfFinPainting`
  (bind _points (`self.CalculatePoints`))
  (bind _returnvalue (`GameplayStatics.GetActorOfClass` "/Game/PaintingGame/Blueprints/Game/BP_GameManager.BP_GameManager_C"))
  (if (>= _points (* (`PGGameManager.GetMosaicSize` _returnvalue) (`PGGameManager.GetMosaicSize` _returnvalue)))
    (`self.OnFinPainting`)))

(fn `GenerateTiles`
  (locals (Row :type Integer) (Column :type Integer) (Size :type Integer :default 0))
  (bind _tilesoffset (`self.TilesOffset`))
  (for _array_element (`self.Tiles`)
    (`self.K2_DestroyActor` _array_element))
  (`KismetArrayLibrary.Array_Clear` (`self.Tiles`))
  (set `local.Row` 0)
  (set `local.Column` 0)
  (bind _returnvalue (`GameplayStatics.GetActorOfClass` "/Game/PaintingGame/Blueprints/Game/BP_GameManager.BP_GameManager_C"))
  (bind _output_get (set `local.Size` (`PGGameManager.GetMosaicSize` _returnvalue)))
  (for _ (range (* _output_get _output_get))
    (bind _returnvalue_2 (`|SpawnActorFromClass` "/Game/PaintingGame/Blueprints/Objects/Mosaic/BP_MosaicTile.BP_MosaicTile_C" (`KismetMathLibrary.MakeTransform` (0.0 0.0 0.0)) "AlwaysSpawn" "MultiplyWithRoot" null null))
    (`KismetArrayLibrary.Array_Add` (`self.Tiles`) _returnvalue_2)
    (`self.K2_AttachToActor` _returnvalue_2 self "None" "KeepRelative" "KeepRelative" "KeepRelative" true)
    (`self.K2_SetActorRelativeLocation` _returnvalue_2 (`KismetMathLibrary.MakeVector` (* (`local.Column`) _tilesoffset) 0.0 (* (`local.Row`) _tilesoffset)) false false)
    (add `/Game/PaintingGame/Blueprints/Objects/Mosaic/BP_MosaicTile.OnPaint` _returnvalue_2 (`|CreateDelegate` :!event `CheckIfFinPainting`))
    (bind _result (`/Engine/EditorBlueprintResources/StandardMacros.IncrementInt` (`local.Column`))
      (:`  `
        (if (>= _result (`local.Size`))
          (`/Engine/EditorBlueprintResources/StandardMacros.IncrementInt` (`local.Row`)
            (:`  `
              (set `local.Column` 0)))))))
  (`self.Multicast_SetTextLocation` (`local.Row`)))

(fn `UserConstructionScript`)