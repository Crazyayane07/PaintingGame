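; BP_Player is the player pawn for the painting game, with a head-following camera and a replicated nickname label.
; Each tick it moves the spring arm to the mesh's Head socket.
; On BeginPlay, the locally controlled player sends the GameInstance's saved nickname to the server and hides its own text label.
; The replicated Nickname's OnRep updates that label's text.
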(event `self.ReceiveTick`
  (params (DeltaSeconds :type "Float (single-precision)"))
  ;[0.08333 0 0] Set camera on head location
  (`SceneComponent.K2_SetWorldLocation` (`self.SpingArmComp`) (`self.GetHeadLocation`) false false))

(event `self.ReceiveBeginPlay`
  (`self.SetUp`))

(event `Server_SetPlayerNickname`
  (params (Nickname :type String))
  (set `self.Nickname` Nickname))

(fn `GetHeadLocation`
  (returns (WorldLoc :type "Vector Structure"))
  (return (`SceneComponent.GetSocketLocation` (`self.Mesh`) "Head")))

(fn `OnRep_Nickname`
  (`TextRenderComponent.K2_SetText` (`self.TextRenderComp`) (`KismetTextLibrary.Conv_StringToText` (`self.Nickname`))))

(fn `SetUp`
  (if (`self.IsLocallyControlled`)
    (bind _asbp_game_instance (cast `/Game/PaintingGame/Blueprints/BP_GameInstance` (`GameplayStatics.GetGameInstance`)))
    (`self.Server_SetPlayerNickname` (`/Game/PaintingGame/Blueprints/BP_GameInstance.SavedNickname` _asbp_game_instance))
    (`SceneComponent.SetHiddenInGame` (`self.TextRenderComp`) true false)))

(fn `UserConstructionScript`)