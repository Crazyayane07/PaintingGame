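; Online round manager for the painting game that generates a mosaic and spawns one board per active player, up to four spawn points.
; Server events stage each round with fades, input blockers and a countdown, driving player pawns through client calls.
; Tick pushes remaining time to players.
; EndGame, not called within this graph, regenerates and clears mosaics for the next round or server-travels to the lobby after the last.
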(event `self.EndGame`
  (`self.SetActorTickEnabled` false)
  (bind _result (`/Engine/EditorBlueprintResources/StandardMacros.IncrementInt` (`self.CurrentRound`))
    (:`  `
      (if (>= _result (`self.Rounds`))
        (`KismetSystemLibrary.ExecuteConsoleCommand` "servertravel /Game/PaintingGame/Maps/M_Lobby" null)
        (else
          (bind _asbp_online_game_mode (cast `/Game/PaintingGame/Blueprints/GameModes/BP_OnlineGameMode` (`GameplayStatics.GetGameMode`)))
          (for _array_element (`/Game/PaintingGame/Blueprints/GameModes/BP_OnlineGameMode.GetActivePlayers` _asbp_online_game_mode)
            (bind _asbp_game_player (cast `/Game/PaintingGame/Blueprints/Player/BP_GamePlayer` (`PlayerState.GetPawn` _array_element)))
            (`/Game/PaintingGame/Blueprints/Player/BP_Player.Client_FadeIn` _asbp_game_player)
            (`/Game/PaintingGame/Blueprints/Player/BP_GamePlayer.Client_DestroyGameInfoWidget` _asbp_game_player)
            (`/Game/PaintingGame/Blueprints/Player/BP_GamePlayer.Client_ResetCooldowns` _asbp_game_player))
          (`KismetSystemLibrary.Delay` 2.0)
          (`self.GenerateMosaic`)
          (`self.Server_ClearMosaics`)
          (bind _asbp_online_game_mode_2 (cast `/Game/PaintingGame/Blueprints/GameModes/BP_OnlineGameMode` (`GameplayStatics.GetGameMode`)))
          (for _array_element_2 (`/Game/PaintingGame/Blueprints/GameModes/BP_OnlineGameMode.GetActivePlayers` _asbp_online_game_mode_2)
            (bind _asbp_player (cast `/Game/PaintingGame/Blueprints/Player/BP_Player` (`PlayerState.GetPawn` _array_element_2)))
            (`/Game/PaintingGame/Blueprints/Player/BP_Player.Client_FadeOut` _asbp_player)
            (`/Game/PaintingGame/Blueprints/Player/BP_Player.Client_AddBlocker` _asbp_player self (`|MakeArray` "MOVEMENT" "INTERACTION" :!type "EBlockers Enum")))
          (`KismetSystemLibrary.Delay` 2.0)
          (bind _asbp_online_game_mode_3 (cast `/Game/PaintingGame/Blueprints/GameModes/BP_OnlineGameMode` (`GameplayStatics.GetGameMode`)))
          (for _array_element_3 (`/Game/PaintingGame/Blueprints/GameModes/BP_OnlineGameMode.GetActivePlayers` _asbp_online_game_mode_3)
            (bind _asbp_game_player_2 (cast `/Game/PaintingGame/Blueprints/Player/BP_GamePlayer` (`PlayerState.GetPawn` _array_element_3)))
            (`/Game/PaintingGame/Blueprints/Player/BP_GamePlayer.Client_CreateCountDown` _asbp_game_player_2))
          (`KismetSystemLibrary.Delay` 2.5)
          (bind _asbp_online_game_mode_4 (cast `/Game/PaintingGame/Blueprints/GameModes/BP_OnlineGameMode` (`GameplayStatics.GetGameMode`)))
          (for _array_element_4 (`/Game/PaintingGame/Blueprints/GameModes/BP_OnlineGameMode.GetActivePlayers` _asbp_online_game_mode_4)
            (bind _asbp_game_player_3 (cast `/Game/PaintingGame/Blueprints/Player/BP_GamePlayer` (`PlayerState.GetPawn` _array_element_4)))
            (`/Game/PaintingGame/Blueprints/Player/BP_GamePlayer.Client_CreateInfoWidget` _asbp_game_player_3)
            (`/Game/PaintingGame/Blueprints/Player/BP_Player.Client_RemoveBlocker` _asbp_game_player_3 self))
          (`self.Server_SetUpTimer`))))))

(event `Server_ClearMosaics`
  (for _array_element (`self.Mosaics`)
    (`/Game/PaintingGame/Blueprints/Objects/Mosaic/BP_Mosaic.Server_Clear` _array_element)))

(event `Server_StartGame`
  (set `self.CurrentRound` 0)
  (`KismetSystemLibrary.Delay` 5.0)
  (`self.SpawnMosaics`)
  (bind _asbp_online_game_mode (cast `/Game/PaintingGame/Blueprints/GameModes/BP_OnlineGameMode` (`GameplayStatics.GetGameMode`)))
  (for _array_element (`/Game/PaintingGame/Blueprints/GameModes/BP_OnlineGameMode.GetActivePlayers` _asbp_online_game_mode)
    (bind _asbp_player (cast `/Game/PaintingGame/Blueprints/Player/BP_Player` (`PlayerState.GetPawn` _array_element)))
    (`/Game/PaintingGame/Blueprints/Player/BP_Player.Client_FadeOut` _asbp_player)
    (`/Game/PaintingGame/Blueprints/Player/BP_Player.Client_AddBlocker` _asbp_player self (`|MakeArray` "MOVEMENT" "INTERACTION" :!type "EBlockers Enum")))
  (`KismetSystemLibrary.Delay` 2.0)
  (bind _asbp_online_game_mode_2 (cast `/Game/PaintingGame/Blueprints/GameModes/BP_OnlineGameMode` (`GameplayStatics.GetGameMode`)))
  (for _array_element_2 (`/Game/PaintingGame/Blueprints/GameModes/BP_OnlineGameMode.GetActivePlayers` _asbp_online_game_mode_2)
    (bind _asbp_game_player (cast `/Game/PaintingGame/Blueprints/Player/BP_GamePlayer` (`PlayerState.GetPawn` _array_element_2)))
    (`/Game/PaintingGame/Blueprints/Player/BP_GamePlayer.Client_CreateCountDown` _asbp_game_player))
  (`KismetSystemLibrary.Delay` 2.5)
  (bind _asbp_online_game_mode_3 (cast `/Game/PaintingGame/Blueprints/GameModes/BP_OnlineGameMode` (`GameplayStatics.GetGameMode`)))
  (for _array_element_3 (`/Game/PaintingGame/Blueprints/GameModes/BP_OnlineGameMode.GetActivePlayers` _asbp_online_game_mode_3)
    (bind _asbp_game_player_2 (cast `/Game/PaintingGame/Blueprints/Player/BP_GamePlayer` (`PlayerState.GetPawn` _array_element_3)))
    (`/Game/PaintingGame/Blueprints/Player/BP_Player.Client_RemoveBlocker` _asbp_game_player_2 self)
    (`/Game/PaintingGame/Blueprints/Player/BP_GamePlayer.Client_CreateInfoWidget` _asbp_game_player_2))
  (`self.Server_SetUpTimer`))

(event `self.ReceiveBeginPlay`
  (`self.Server_SetUp`))

(event `self.StartGame`
  (`self.Server_StartGame`))

(event `Server_SetUp`
  (`self.GenerateMosaic`)
  (`self.StartGame`))

(event `Server_SetUpTimer`
  (set `self.StartGameTime` (`GameplayStatics.GetTimeSeconds`))
  (`self.SetActorTickEnabled` true))

(event `self.ReceiveTick`
  (params (DeltaSeconds :type "Float (single-precision)"))
  (`parent.ReceiveTick` DeltaSeconds)
  (`self.Server_Tick`))

(event `SpawnMosaics`
  (bind _asbp_online_game_mode (cast `/Game/PaintingGame/Blueprints/GameModes/BP_OnlineGameMode` (`GameplayStatics.GetGameMode`)))
  (for (_array_element _array_index) (`|MakeArray` (`self.SpawnMosaicLocation1`) (`self.SpawnMosaicLocation2`) (`self.SpawnMosaicLocation3`) (`self.SpawnMosaicLocation4`))
    (bind _activeplayers (`/Game/PaintingGame/Blueprints/GameModes/BP_OnlineGameMode.GetActivePlayers` _asbp_online_game_mode))
    (if (< _array_index (`KismetArrayLibrary.Array_Length` _activeplayers))
      (bind _returnvalue (`|SpawnActorFromClass` "/Game/PaintingGame/Blueprints/Objects/Mosaic/BP_Mosaic.BP_Mosaic_C" (`SceneComponent.K2_GetComponentToWorld` _array_element) "Undefined" "MultiplyWithRoot" null (`|GetArrayItem` _activeplayers _array_index) null))
      (`KismetArrayLibrary.Array_Add` (`self.Mosaics`) _returnvalue)
      (else
        (break)))))

(event `Server_Tick`
  (bind _asbp_online_game_mode (cast `/Game/PaintingGame/Blueprints/GameModes/BP_OnlineGameMode` (`GameplayStatics.GetGameMode`)))
  (for _array_element (`/Game/PaintingGame/Blueprints/GameModes/BP_OnlineGameMode.GetActivePlayers` _asbp_online_game_mode)
    (bind _asbp_game_player (cast `/Game/PaintingGame/Blueprints/Player/BP_GamePlayer` (`PlayerState.GetPawn` _array_element)))
    (`/Game/PaintingGame/Blueprints/Player/BP_GamePlayer.Client_UpdateTimerText` _asbp_game_player (- (`self.GameDuration`) (- (`GameplayStatics.GetTimeSeconds`) (`self.StartGameTime`))))))

(fn `UserConstructionScript`
  (`parent.UserConstructionScript`))