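; BP_GamePlayer is the painting game's player, handling object interaction, brush color and HUD updates.
; Each Tick line-traces from the head along control rotation to cache a BPI_InteractableObject actor, which only a non-interactable hit clears, not a miss.
; TryInteract messages that actor unless interaction is blocked, and SetNewBrushColor stores the color ID and passes it to the child-actor BP_Brush.
; Client events forward countdown, info widget and timer updates to BP_GameHUD.
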(event `self.ReceiveTick`
  (params (DeltaSeconds :type "Float (single-precision)"))
  (`parent.ReceiveTick` DeltaSeconds)
  (`self.TraceForInteractableObject`))

(event `self.TryInteract`
  (if (not (`self.IsBlocking` (enumliteral `EBlockers` "INTERACTION")))
    (bind _interactableobjectinrange (`self.InteractableObjectInRange`)
      (:`then`
        (message `/Game/PaintingGame/Blueprints/Objects/BPI_InteractableObject.Interact` _interactableobjectinrange self))
      (:`else`))))

(event `Client_CreateCountDown`
  (bind _asbp_game_hud (cast `/Game/PaintingGame/Blueprints/HUD/BP_GameHUD` (`PlayerController.GetHUD` (`GameplayStatics.GetPlayerController` 0))))
  (`/Game/PaintingGame/Blueprints/HUD/BP_GameHUD.CreateCountdown` _asbp_game_hud))

(event `Client_CreateInfoWidget`
  (bind _asbp_game_hud (cast `/Game/PaintingGame/Blueprints/HUD/BP_GameHUD` (`PlayerController.GetHUD` (`GameplayStatics.GetPlayerController` 0))))
  (`/Game/PaintingGame/Blueprints/HUD/BP_GameHUD.CreateGameInfoWidget` _asbp_game_hud))

(event `Client_UpdateTimerText`
  (params (NewTime :type "Float (double-precision)"))
  (bind _asbp_game_hud (cast `/Game/PaintingGame/Blueprints/HUD/BP_GameHUD` (`PlayerController.GetHUD` (`GameplayStatics.GetPlayerController` 0))))
  (`/Game/PaintingGame/Blueprints/HUD/BP_GameHUD.UpdateTimerText` _asbp_game_hud NewTime))

(fn `GetCurrentColorId`
  (returns (Id :type Integer))
  (return (`self.CurrentColorId`)))

(fn `SetNewBrushColor`
  (params (ColorId :type Integer))
  (bind _output_get (set `self.CurrentColorId` ColorId))
  (bind _asbp_brush (cast `/Game/PaintingGame/Blueprints/Objects/BP_Brush` (`ChildActorComponent.ChildActor` (`self.Brush`))))
  (`/Game/PaintingGame/Blueprints/Objects/BP_Brush.SetNewBrushColor` _asbp_brush _output_get))

(fn `TraceForInteractableObject`
  (bind _worldloc (`self.GetHeadLocation`))
  (bind (_outhit _returnvalue) (`KismetSystemLibrary.LineTraceSingleForObjects` _worldloc (+ _worldloc (* (`KismetMathLibrary.GetForwardVector` (`self.GetControlRotation`)) (`self.InteractionDistance`))) (`self.InteractableObjects`)))
  (if _returnvalue
    (bind (_bblockinghit _binitialoverlap _time _distance _location _impactpoint _normal _impactnormal _physmat _hitactor) (`GameplayStatics.BreakHitResult` _outhit))
    (if (`KismetSystemLibrary.DoesImplementInterface` _hitactor "/Game/PaintingGame/Blueprints/Objects/BPI_InteractableObject.BPI_InteractableObject_C")
      (set `self.InteractableObjectInRange` _hitactor)
      (else
        (set `self.InteractableObjectInRange` null)))))

(fn `UserConstructionScript`
  (`parent.UserConstructionScript`))