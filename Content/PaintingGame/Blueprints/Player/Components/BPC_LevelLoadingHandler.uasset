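; Player controller component that handles screen fade transitions around level loading in the painting game.
; On local BeginPlay it creates a cached, initially fully faded WBP_ScreenFader.
; FadeOutForLevel reveals the level, blocking movement and interaction through the pawn's PGBlockerHandlerComponent until the animation ends, then signals completion.
; OpenLevel stores the level and options, applies the same blockers, fades in the cover, then opens the level by name.
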(event `FadeOutForLevel`
  (bind (_bhasblocker _blockerhandler) (`self.GetBlockerHandler`))
  (if _bhasblocker
    (`PGBlockerHandlerComponent.AddBlocker` _blockerhandler self (`|MakeArray` "MOVEMENT" "INTERACTION" :!type "EBlockers Enum")))
  (bind _screenfaderref (`self.GetScreenFader`))
  (add `/Game/PaintingGame/Widgets/WBP_ScreenFader.OnAnimFin` _screenfaderref (delegate `OnFadedOut`))
  (`/Game/PaintingGame/Widgets/WBP_ScreenFader.StartFadingOut` _screenfaderref))

(event `OnFadedOut`
  (bind _screenfaderref (`self.GetScreenFader`))
  (remove `/Game/PaintingGame/Widgets/WBP_ScreenFader.OnAnimFin` _screenfaderref (delegate `OnFadedOut`))
  (bind (_bhasblocker _blockerhandler) (`self.GetBlockerHandler`))
  (if _bhasblocker
    (`PGBlockerHandlerComponent.RemoveBlocker` _blockerhandler self))
  (`self.OnFadeOutFin`))

(event `OpenLevel`
  (params (Level :type Name) (NextLevelOptions :type String))
  (set `self.NextLevelToLoad` Level)
  (set `self.Next LevelOptions` NextLevelOptions)
  (bind _screenfaderref (`self.GetScreenFader`))
  (add `/Game/PaintingGame/Widgets/WBP_ScreenFader.OnAnimFin` _screenfaderref (delegate `OnFinFadeIn`))
  (`self.StartFadingIn`))

(event `OnFinFadeIn`
  (bind _screenfaderref (`self.GetScreenFader`))
  (remove `/Game/PaintingGame/Widgets/WBP_ScreenFader.OnAnimFin` _screenfaderref (delegate `OnFinFadeIn`))
  (`GameplayStatics.OpenLevel` (`self.NextLevelToLoad`) true (`self.Next LevelOptions`)))

(event `StartFadingIn`
  (bind (_bhasblocker _blockerhandler) (`self.GetBlockerHandler`))
  (if _bhasblocker
    (`PGBlockerHandlerComponent.AddBlocker` _blockerhandler self (`|MakeArray` "MOVEMENT" "INTERACTION" :!type "EBlockers Enum")))
  (bind _screenfaderref (`self.GetScreenFader`))
  (`/Game/PaintingGame/Widgets/WBP_ScreenFader.StartFadingIn` _screenfaderref))

(event `self.ReceiveBeginPlay`
  (bind _asplayer_controller (cast `PlayerController` (`self.GetOwner`)))
  (if (`Controller.IsLocalPlayerController` _asplayer_controller)
    (`self.GetScreenFader`)))

(fn `GetBlockerHandler`
  (returns (bHasBlocker :type Boolean) (BlockerHandler :type "PGBlockerHandlerComponent Object Reference"))
  (bind _blockerhandlerref (`self.BlockerHandlerRef`)
    (:`then`
      (return true _blockerhandlerref))
    (:`else`
      (bind _asplayer_controller (cast `PlayerController` (`self.GetOwner`))
        (:`then`
          (bind _returnvalue (`Actor.GetComponentByClass` (`Controller.K2_GetPawn` _asplayer_controller) "/Script/PaintingGame.PGBlockerHandlerComponent"))
          (`/Engine/EditorBlueprintResources/StandardMacros.IsValid` _returnvalue
            (:`Is Valid`
              (bind _output_get (set `self.BlockerHandlerRef` _returnvalue))
              (return true _output_get))
            (:`Is Not Valid`
              (return false null))))
        (:`CastFailed`
          (return false null))))))

(fn `GetScreenFader`
  (returns (ScreenFaderRef :type "/Game/PaintingGame/Widgets/WBP_ScreenFader Object Reference"))
  (bind _screenfaderref (`self.ScreenFaderRef`)
    (:`then`
      (return _screenfaderref))
    (:`else`
      (bind _asplayer_controller (cast `PlayerController` (`self.GetOwner`)))
      (bind _returnvalue (`|CreateWidget` "/Game/PaintingGame/Widgets/WBP_ScreenFader.WBP_ScreenFader_C" _asplayer_controller true))
      (bind _output_get (set `self.ScreenFaderRef` _returnvalue))
      (`UserWidget.AddToViewport` _output_get 0)
      (return _output_get))))