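; BP_ColorableObject is a painting game object whose mesh can be recolored by palette ID.
; SetNewColor lazily finds and caches BP_GameManager, then checks the requested ID against its AllowedColors array.
; For a valid ID, it stores the ColorId and applies a new M_MeshColor dynamic material instance to slot 0 of the supplied mesh, setting its Color parameter.
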(fn `Set New Color`
  (params (MeshComp :type "PrimitiveComponent Object Reference") (NewColorId :type Integer))
  (bind _allowedcolors (`PGGameManager.AllowedColors` (`self.GameManagerRef`)))
  (`self.GameManagerRef`
    (:`then`
      _)
    (:`else`
      (bind _returnvalue (`GameplayStatics.GetActorOfClass` "/Game/PaintingGame/Blueprints/Game/BP_GameManager.BP_GameManager_C"))
      (set `self.GameManagerRef` _returnvalue)))
  (if (`KismetArrayLibrary.Array_IsValidIndex` _allowedcolors NewColorId)
    (set `self.ColorId` NewColorId)
    (bind _returnvalue_2 (`PrimitiveComponent.CreateDynamicMaterialInstance` MeshComp 0 "/Game/PaintingGame/Materials/M_MeshColor.M_MeshColor" "None"))
    (`MaterialInstanceDynamic.SetVectorParameterValue` _returnvalue_2 "Color" (`|GetArrayItem` _allowedcolors NewColorId))))

(fn `UserConstructionScript`)