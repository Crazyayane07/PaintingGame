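; BP_PaintBucket is an interactable paint bucket that sets the interacting player's brush to the bucket's color ID.
; Its construction script looks up that ID in BP_GameManager's allowed colors and tints the paint mesh through a dynamic material instance.
; Entering or leaving interaction range toggles an outline overlay material on both meshes, only for the locally controlled player.
; It also exposes a cooldown duration through a getter.
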(event `/Game/PaintingGame/Blueprints/Objects/BPI_InteractableObject.Interact`
  (params (PlayerInstigator :type "/Game/PaintingGame/Blueprints/Player/BP_GamePlayer Object Reference"))
  (`/Game/PaintingGame/Blueprints/Player/BP_GamePlayer.SetNewBrushColor` PlayerInstigator (`self.ColorId`)))

(event `/Game/PaintingGame/Blueprints/Objects/BPI_InteractableObject.OnInteractionInRange`
  (params (PlayerInstigator :type "/Game/PaintingGame/Blueprints/Player/BP_GamePlayer Object Reference"))
  (if (`Pawn.IsLocallyControlled` PlayerInstigator)
    (`self.Client_ActivateOverlay` true)))

(event `/Game/PaintingGame/Blueprints/Objects/BPI_InteractableObject.OnInteractionOutOfRange`
  (params (PlayerInstigator :type "/Game/PaintingGame/Blueprints/Player/BP_GamePlayer Object Reference"))
  (if (`Pawn.IsLocallyControlled` PlayerInstigator)
    (`self.Client_ActivateOverlay` false)))

(event `Client_ActivateOverlay`
  (params (bActivate :type Boolean))
  (`MeshComponent.SetOverlayMaterial` (`self.SM_Bucket`) (select `bool` bActivate :`true` "/Game/PaintingGame/Materials/MI_Outline.MI_Outline" :!type "MaterialInterface Object Reference"))
  (`MeshComponent.SetOverlayMaterial` (`self.SM_Paint`) (select `bool` bActivate :`true` "/Game/PaintingGame/Materials/MI_Outline.MI_Outline" :!type "MaterialInterface Object Reference")))

(fn `GetCooldownDuration`
  (returns (CooldownDuration :type "Float (double-precision)"))
  (return (`self.CooldownDuration`)))

(fn `UserConstructionScript`
  (bind _returnvalue (`GameplayStatics.GetActorOfClass` "/Game/PaintingGame/Blueprints/Game/BP_GameManager.BP_GameManager_C"))
  (bind _returnvalue_2 (`PrimitiveComponent.CreateDynamicMaterialInstance` (`self.SM_Paint`) 0 "/Game/PaintingGame/Materials/M_MeshColor.M_MeshColor" "None"))
  (`MaterialInstanceDynamic.SetVectorParameterValue` _returnvalue_2 "Color" (`|GetArrayItem` (`PGGameManager.AllowedColors` _returnvalue) (`self.ColorId`))))