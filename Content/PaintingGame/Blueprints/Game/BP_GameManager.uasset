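; Game manager for the painting game that generates a mosaic and controls match start and end.
; On BeginPlay it blocks every player's movement and interaction, then triggers a level fade-out.
; The fade's completion starts a HUD countdown, which then shows game info, unblocks player 0, records the start time and enables tick.
; EndGame disables tick and returns to the main menu after a short delay.
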(event `self.StartGame`
  (for _array_element (`GameStateBase.PlayerArray` (`GameplayStatics.GetGameState`))
    (bind _returnvalue (`PlayerState.GetPawn` _array_element))
    (`PGBlockerHandlerComponent.AddBlocker` (`self.GetComponentByClass` _returnvalue "/Script/PaintingGame.PGBlockerHandlerComponent") self (`|MakeArray` "MOVEMENT" "INTERACTION" :!type "EBlockers Enum"))
    (bind _returnvalue_2 (`self.GetComponentByClass` (`Pawn.GetLocalViewingPlayerController` _returnvalue) "/Game/PaintingGame/Blueprints/Player/Components/BPC_LevelLoadingHandler.BPC_LevelLoadingHandler_C"))
    (add `/Game/PaintingGame/Blueprints/Player/Components/BPC_LevelLoadingHandler.OnFadeOutFin` _returnvalue_2 (delegate `OnPlayerFadeOutFin`))
    (`/Game/PaintingGame/Blueprints/Player/Components/BPC_LevelLoadingHandler.FadeOutForLevel` _returnvalue_2)))

(event `OnPlayerFadeOutFin`
  (bind _asbp_game_hud (cast `/Game/PaintingGame/Blueprints/HUD/BP_GameHUD` (`PlayerController.GetHUD` (`GameplayStatics.GetPlayerController` 0))))
  (bind _countdownref (`/Game/PaintingGame/Blueprints/HUD/BP_GameHUD.CreateCountdown` _asbp_game_hud))
  (add `/Game/PaintingGame/Widgets/WBP_Countdown.OnFinCountdown` _countdownref (delegate `OnFinCountdown`)))

(event `OnFinCountdown`
  (bind _asbp_game_hud (cast `/Game/PaintingGame/Blueprints/HUD/BP_GameHUD` (`PlayerController.GetHUD` (`GameplayStatics.GetPlayerController` 0))))
  (`/Game/PaintingGame/Blueprints/HUD/BP_GameHUD.CreateGameInfoWidget` _asbp_game_hud)
  (`PGBlockerHandlerComponent.RemoveBlocker` (`self.GetComponentByClass` (`GameplayStatics.GetPlayerPawn` 0) "/Script/PaintingGame.PGBlockerHandlerComponent") self)
  (set `self.StartGameTime` (`GameplayStatics.GetTimeSeconds`))
  (`self.SetActorTickEnabled` true))

(event `self.EndGame`
  (`self.SetActorTickEnabled` false)
  (`KismetSystemLibrary.Delay` 1.0)
  (`/Game/PaintingGame/Blueprints/BP_PaintingGameLibrary.OpenLevel` "M_MainMenu"))

(event `self.ReceiveBeginPlay`
  (`self.GenerateMosaic`)
  (`self.StartGame`))

(fn `UserConstructionScript`)